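; Player combat component for BP_ThirdPersonCharacter, handling target lock-on, directional dodge and sword combos.
; Lock-on sphere-traces for a pawn, attaches a marker actor and steers control rotation toward it each tick.
; Dodge picks a montage from the player's WASD key and sets an i-frame flag, while attack montage notifies end the combo unless input is buffered.
; Damage trace events run a looping timer that sweeps hilt to tip, throttling hits with a delayed DoOnce.
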(event `self.ReceiveBeginPlay`
  ;[0.15 0.02017 0.01768 0.5] Get Player Class
  (bind _asbp_third_person_character (cast `/Game/ThirdPerson/Blueprints/BP_ThirdPersonCharacter` (`self.GetOwner`)))
  (set `self.playerBP` _asbp_third_person_character)
  (set `self.swordDamage` 20.0))

(event `EnhancedInput|/Game/ThirdPerson/Input/Actions/IA_Lock`
  (params (ActionValue :type Boolean) (ElapsedSeconds :type "Float (double-precision)") (TriggeredSeconds :type "Float (double-precision)") (InputAction :type "InputAction Object Reference" :default "/Game/ThirdPerson/Input/Actions/IA_Lock.IA_Lock"))
  (bind _playerbp (`self.playerBP`))
  (bind _returnvalue (`Actor.K2_GetActorLocation` _playerbp))
  (bind (_returnvalue_location _returnvalue_rotation) (`KismetMathLibrary.BreakTransform` (`Actor.GetTransform` (`self.lockedOnTarget`))))
  (bind _charactermovement (`Character.CharacterMovement` (`self.playerBP`)))
  (bind _charactermovement_2 (`Character.CharacterMovement` (`self.playerBP`)))
  (bind (_returnvalue_x _returnvalue_y) (`KismetMathLibrary.BreakVector` (`KismetMathLibrary.GetForwardVector` (`SceneComponent.K2_GetComponentRotation` (`PlayerCameraManager.TransformComponent` (`GameplayStatics.GetPlayerCameraManager` 0))))))
  ;[0.15 0 0.1433 0.5] Target Lockon
  (:`Started`
    (`self.lockedOnTarget`
      (:`then`
        (set `self.lockedOnTarget` null)
        (set `CharacterMovementComponent.bOrientRotationToMovement` true _charactermovement)
        (set `CharacterMovementComponent.bUseControllerDesiredRotation` false _charactermovement)
        (`Actor.K2_DestroyActor` (`self.lockedWidget`)))
      (:`else`
        (bind (_outhit _returnvalue_2) (`KismetSystemLibrary.SphereTraceSingleForObjects` :`Start` (+ _returnvalue (* (`Actor.GetActorForwardVector` _playerbp) (500.0 500.0 0.0))) :`End` (+ _returnvalue (* (`KismetMathLibrary.MakeVector` _returnvalue_x _returnvalue_y) 1000.0)) :`Radius` 500.0 :`ObjectTypes` (`|MakeArray` "ObjectTypeQuery3" :!type "EObjectTypeQuery Enum") :`DrawDebugType` "ForDuration" :`DrawTime` 2.0))
        (if _returnvalue_2
          (set `self.lockedOnTarget` (`.HitActor` (`GameplayStatics.BreakHitResult` _outhit)))
          (set `CharacterMovementComponent.bOrientRotationToMovement` false _charactermovement_2)
          (set `CharacterMovementComponent.bUseControllerDesiredRotation` true _charactermovement_2)
          (bind _returnvalue_3 (`|SpawnActorFromClass` "/Game/BluePrint/BP_TargetLockWidget.BP_TargetLockWidget_C" (`KismetMathLibrary.MakeTransform` _returnvalue_location _returnvalue_rotation) "AlwaysSpawn" "MultiplyWithRoot" null null))
          (bind _output_get (set `self.lockedWidget` _returnvalue_3))
          (`Actor.K2_AttachToActor` _output_get (`self.lockedOnTarget`) "None" "SnapToTarget" "KeepRelative" "KeepRelative" true))))))

(event `self.ReceiveTick`
  (params (DeltaSeconds :type "Float (single-precision)"))
  (bind _playerbp (`self.playerBP`))
  (bind (_returnvalue_roll _returnvalue_pitch _returnvalue_yaw) (`KismetMathLibrary.BreakRotator` (`KismetMathLibrary.FindLookAtRotation` (`Actor.K2_GetActorLocation` _playerbp) (`Actor.K2_GetActorLocation` (`self.lockedOnTarget`)))))
  ;[0.15 0 0.1433 0.5] Target Lockon
  ;;[0.15 0 0.1433 0.5] Update
  (`self.lockedOnTarget`
    (:`then`
      (`Controller.SetControlRotation` (`Pawn.GetController` _playerbp) (`KismetMathLibrary.MakeRotator` _returnvalue_roll (- _returnvalue_pitch 15.0) _returnvalue_yaw)))
    (:`else`)))

(event `EnhancedInput|/Game/ThirdPerson/Input/Actions/IA_Dodge`
  (params (ActionValue :type Boolean) (ElapsedSeconds :type "Float (double-precision)") (TriggeredSeconds :type "Float (double-precision)") (InputAction :type "InputAction Object Reference" :default "/Game/ThirdPerson/Input/Actions/IA_Dodge.IA_Dodge"))
  (:`Started`
    (if (`self.canDodge?`)
      (`|ExecutionSequence`
        (:`then_0`
          (if (`CharacterMovementComponent.bUseControllerDesiredRotation` (`Character.CharacterMovement` (`self.playerBP`)))
            _
            (else
              _))
          (switch `string` (`KismetTextLibrary.Conv_TextToString` (`KismetInputLibrary.Key_GetDisplayName` (`/Game/ThirdPerson/Blueprints/BP_ThirdPersonCharacter.Direction Key` (`self.playerBP`))))
            (:`W`
              (set `self.movementDirection` "NewEnumerator0"))
            (:`A`
              (set `self.movementDirection` "NewEnumerator1"))
            (:`S`
              (set `self.movementDirection` "NewEnumerator2"))
            (:`D`
              (set `self.movementDirection` "NewEnumerator3"))))
        (:`then_1`
          (`|PlayMontage` (`Character.Mesh` (`self.playerBP`)) (select `/Game/BluePrint/BPE_MovementDirection` (`self.movementDirection`) :`NewEnumerator0` "/Game/Characters/Souls/Combat/combat_animation/Dodge/Dodge_F_Montage.Dodge_F_Montage" :`NewEnumerator1` "/Game/Characters/Souls/Combat/combat_animation/Dodge/Dodge_L_Montage.Dodge_L_Montage" :`NewEnumerator2` "/Game/Characters/Souls/Combat/combat_animation/Dodge/Dodge_B_Montage.Dodge_B_Montage" :`NewEnumerator3` "/Game/Characters/Souls/Combat/combat_animation/Dodge/Dodge_R_Montage.Dodge_R_Montage" :!type "AnimMontage Object Reference")
            (:`then`
              (set `self.canDodge?` false)
              (set `self.isIframe?` true))
            (:`OnCompleted`
              (set `self.isIframe?` false :!label _label)
              (`KismetSystemLibrary.Delay` 0.1)
              (set `self.canDodge?` true))
            (:`OnInterrupted`
              (goto _label))))))))

(event `EnhancedInput|/Game/ThirdPerson/Input/Actions/IA_Attack`
  (params (ActionValue :type Boolean) (ElapsedSeconds :type "Float (double-precision)") (TriggeredSeconds :type "Float (double-precision)") (InputAction :type "InputAction Object Reference" :default "/Game/ThirdPerson/Input/Actions/IA_Attack.IA_Attack"))
  ;[1 0 0 0.5] Combo Attack Animation
  (:`Started`
    (if (`self.isAttacking?`)
      (set `self.canKeepAttacking?` true)
      (else
        (set `self.isAttacking?` true)
        (`|PlayMontage` (`Character.Mesh` (`self.playerBP`)) "/Game/Characters/Souls/Combat/combat_animation/ANM_Attack.ANM_Attack"
          (:`OnCompleted`
            (set `self.isAttacking?` false :!label _label_2)
            (set `self.canKeepAttacking?` false))
          (:`OnInterrupted`
            (goto _label_2))
          (:`OnNotifyBegin`
            (if (and (`self.isAttacking?`) (`self.canKeepAttacking?`))
              (set `self.canKeepAttacking?` false)
              (else
                (`AnimInstance.Montage_Stop` (`SkeletalMeshComponent.GetAnimInstance` (`Character.Mesh` (`self.playerBP`))) 0.2 "/Game/Characters/Souls/Combat/combat_animation/ANM_Attack.ANM_Attack")))))))))

(event `EndDamageTrace`
  ;[1 0 0 0.5] SwordTrace
  (if (`KismetSystemLibrary.K2_IsValidTimerHandle` (stale `BeginDamageTrace` _returnvalue))
    (`KismetSystemLibrary.K2_ClearAndInvalidateTimerHandle` (stale `BeginDamageTrace` _returnvalue))))

(event `BeginDamageTrace`
  ;[1 0 0 0.5] SwordTrace
  (bind _returnvalue (`KismetSystemLibrary.K2_SetTimerDelegate` (delegate `DamageTrace`) 0.01 true)))

(event `DamageTrace`
  (bind _playerbp (`self.playerBP`))
  ;[1 0 0 0.5] SwordTrace
  (bind (_outhit _returnvalue) (`KismetSystemLibrary.SphereTraceSingleForObjects` :`Start` (`SceneComponent.K2_GetComponentLocation` (`/Game/ThirdPerson/Blueprints/BP_ThirdPersonCharacter.SwordHandlePos` _playerbp)) :`End` (`SceneComponent.K2_GetComponentLocation` (`/Game/ThirdPerson/Blueprints/BP_ThirdPersonCharacter.SwordTipPos` _playerbp)) :`Radius` 20.0 :`ObjectTypes` (`|MakeArray` "ObjectTypeQuery3" :!type "EObjectTypeQuery Enum") :`DrawDebugType` "ForDuration"))
  (if _returnvalue
    (`/Engine/EditorBlueprintResources/StandardMacros.DoOnce` false :!label _label_3
      (:`Completed`
        (`GameplayStatics.ApplyDamage` (`.HitActor` (`GameplayStatics.BreakHitResult` _outhit)) (`self.swordDamage`) null (`self.playerBP`))
        (`KismetSystemLibrary.Delay` 0.2)
        (goto _label_3 :!via `Reset`)))))