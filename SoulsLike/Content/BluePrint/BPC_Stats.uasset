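; BPC_Stats is a stats component that tracks its owner's health and signals death.
; IncreaseValue adds a value to Health, clamped between zero and MaxHealth, then calls Die at zero, which sends DieMessage to the owner.
; It also updates a health progress bar, supplied through SetHealthProgressBar, with the health fraction when that widget is valid.
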(event `Die`
  (message `/Game/BluePrint/BPI_Damage.Die` (`self.GetOwner`)))

(event `SetHealthProgressBar`
  (params (healthProgressBar :type "ProgressBar Object Reference"))
  (set `self.Health Progress Bar` healthProgressBar))

(fn `increaseValue`
  (params (Stat :type "/Game/BluePrint/BPE_Stats Enum" :default "NewEnumerator0") (Value :type "Float (double-precision)"))
  (bind _maxhealth (`self.maxHealth`))
  (switch `/Game/BluePrint/BPE_Stats` Stat
    (:`NewEnumerator0`
      (bind _output_get (set `self.health` (`KismetMathLibrary.FClamp` (+ (`self.health`) Value) 0.0 _maxhealth)))
      (`|ExecutionSequence`
        (:`then_0`
          (if (<= _output_get 0.0)
            (`self.Die`)))
        (:`then_1`
          (bind _health_progress_bar (`self.Health Progress Bar`)
            (:`then`
              (`ProgressBar.SetPercent` _health_progress_bar (/ _output_get _maxhealth)))
            (:`else`)))))))